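; BP_Button1 is a pressable button actor that asks BP_ThirdPersonGameMode to spawn Turtle 1 when the player interacts with it.
; A box overlap with BP_ThirdPersonCharacter opens a gate, so the Interact input only works while the character stands in range.
; Each press also plays a Bricks sound and runs two chained timelines that lerp the button mesh in and back out between transforms cached at BeginPlay.
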(event OnComponentBeginOverlap(Box)
  (params (OverlappedComponent :type Primitive%20Component%20Object%20Reference) (OtherActor :type Actor%20Object%20Reference) (OtherComp :type Primitive%20Component%20Object%20Reference) (OtherBodyIndex :type Integer) (bFromSweep :type Boolean) (SweepResult :type Hit%20Result%20Structure%20%28by%20ref%29))
  ;[1 1 1] Interaction
  (Utilities|Casting|CastToBP_ThirdPersonCharacter OtherActor)
  (Utilities|FlowControl|Gate true) ; enters at Open
)

(event OnComponentEndOverlap(Box)
  (params (OverlappedComponent :type Primitive%20Component%20Object%20Reference) (OtherActor :type Actor%20Object%20Reference) (OtherComp :type Primitive%20Component%20Object%20Reference) (OtherBodyIndex :type Integer))
  ;[1 1 1] Interaction
  (Utilities|Casting|CastToBP_ThirdPersonCharacter OtherActor)
  (Utilities|FlowControl|Gate true) ; enters at Close
)

(event EventBeginPlay
  (bind _button (Variables|Default|GetButton))
  (bind _returnvalue (Transformation|GetRelativeTransform _button))
  ;[1 1 1] Button
  (Variables|Default|SetButton%20Off (Math|Transform|MakeTransform (.location _returnvalue) (.rotation _returnvalue) (.scale _returnvalue)))
  (Variables|Default|SetButton%20On (Math|Transform|MakeTransform (- (.location _returnvalue) "10.000000,0.000000,0.000000") (.rotation _returnvalue) (.scale _returnvalue)))
  (Input|EnableInput (Game|GetPlayerController 0)))

(event Input|ActionEvents|InputActionInteract1
  (params (Key :type Key%20Structure))
  ;[1 1 1] Interaction
  (:Pressed
    (Utilities|FlowControl|Gate true
      (:Exit
        (Utilities|FlowControl|Sequence
          (:then_0
            ;[1 1 1] Event
            (bind _asbp_third_person_game_mode (Utilities|Casting|CastToBP_ThirdPersonGameMode (Game|GetGameMode)))
            (Default|SpawnTurtle1 _asbp_third_person_game_mode))
          (:then_1
            ;[1 1 1] Animation
            (Audio|PlaySoundatLocation "/Game/Core/Sounds/bricks.bricks" (Transformation|GetActorLocation) "0, 0, 0" 1.0 1.0 0.0 0 0 0 0)
            (bind _button_in (Timeline|Button%20In PlayFromStart)
              (:Update
                (Transformation|SetRelativeTransform (Variables|Default|GetButton) (Math|Transform|Lerp(Transform) (Variables|Default|GetButton%20Off) (Variables|Default|GetButton%20On) _button_in) false false))
              (:Finished
                (bind _button_in_2 (Timeline|Button%20Out ReverseFromEnd)
                  (:Update
                    (Transformation|SetRelativeTransform (Variables|Default|GetButton) (Math|Transform|Lerp(Transform) (Variables|Default|GetButton%20Off) (Variables|Default|GetButton%20On) _button_in_2) false false)))))))))))

(fn ConstructionScript)