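; BP_Button is an interactable button actor that plays a sound and animates a press when its Interact event fires.
; At BeginPlay it caches resting and pressed relative transforms, offset along X, and enables input for the first player controller.
; Interact runs one timeline to lerp the Button component inward, then reverses a second timeline to return it.
; The file wires no gameplay effect to the press.
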(event Custom|Interact
  ;[1 1 1] Animation
  (Audio|PlaySoundatLocation "/Game/Core/Sounds/bricks.bricks" (Transformation|GetActorLocation) "0, 0, 0" 1.0 1.0 0.0 0 0 0 0)
  (bind _button_in (Timeline|Timeline PlayFromStart)
    (:Update
      (Transformation|SetRelativeTransform (Variables|Default|GetButton) (Math|Transform|Lerp(Transform) (Variables|Default|GetButton%20Off) (Variables|Default|GetButton%20On) _button_in) false false))
    (:Finished
      (bind _button_in_2 (Timeline|Timeline_0 ReverseFromEnd)
        (:Update
          (Transformation|SetRelativeTransform (Variables|Default|GetButton) (Math|Transform|Lerp(Transform) (Variables|Default|GetButton%20Off) (Variables|Default|GetButton%20On) _button_in_2) false false))))))

(event EventBeginPlay
  (bind _button (Variables|Default|GetButton))
  (bind _returnvalue (Transformation|GetRelativeTransform _button))
  ;[1 1 1] Button
  (Variables|Default|SetButton%20Off (Math|Transform|MakeTransform (.location _returnvalue) (.rotation _returnvalue) (.scale _returnvalue)))
  (Variables|Default|SetButton%20On (Math|Transform|MakeTransform (- (.location _returnvalue) "10.000000,0.000000,0.000000") (.rotation _returnvalue) (.scale _returnvalue)))
  (Input|EnableInput (Game|GetPlayerController 0)))

(fn ConstructionScript)

(fn NewFunction)